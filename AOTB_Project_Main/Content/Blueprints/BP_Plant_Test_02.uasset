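; BP_Plant_Test_02 is a test plant actor that replaces itself with BP_Plant_Test_03, apparently as a growth stage.
; When the third-person character overlaps its PlayerInputBox, it sets IsNeedsMet and waits a short delay.
; It then spawns the next plant at its own location, regardless of collision, and destroys itself.
; A disconnected spawn-and-destroy chain never runs.
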(event OnComponentBeginOverlap(PlayerInputBox)
  (params (OverlappedComponent :type Primitive%20Component%20Object%20Reference) (OtherActor :type Actor%20Object%20Reference) (OtherComp :type Primitive%20Component%20Object%20Reference) (OtherBodyIndex :type Integer) (bFromSweep :type Boolean) (SweepResult :type Hit%20Result%20Structure%20%28by%20ref%29))
  (Utilities|Casting|CastToBP_ThirdPersonCharacter OtherActor)
  (Variables|Default|SetIsNeedsMet true)
  (Utilities|FlowControl|Delay 5.0)
  (Game|SpawnActorfromClass "/Game/Blueprints/BP_Plant_Test_03.BP_Plant_Test_03_C" (Math|Conversions|ToTransform(Vector) (Transformation|GetActorLocation self)) "AlwaysSpawn" "MultiplyWithRoot" 0 0)
  (Actor|DestroyActor self))

(event EventBeginPlay)

(event Collision|EventActorBeginOverlap
  (params (OtherActor :type Actor%20Object%20Reference)))

(event EventTick
  (params (DeltaSeconds :type Float%20%28single-precision%29)))

(fn ConstructionScript)